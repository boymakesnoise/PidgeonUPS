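; BP_Pickup is a collectible that the player character gathers by touching it.
; It spins by adding a fixed yaw rotation to its Scene component every tick, so the speed depends on frame rate.
; When a BP_Character overlaps its Box, it increments that character's Pickups count and destroys itself.
; BeginPlay caches the player character in PlayerRef, which the graph never reads.
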(event `self.ReceiveTick`
  (params (DeltaSeconds :type "Float (single-precision)"))
  (`SceneComponent.K2_AddRelativeRotation` (`self.Scene`) (struct :`Yaw` 2.0) false false))

(event `self.ReceiveBeginPlay`
  (bind _asbp_character (cast `/Game/Blueprints/BP_Character` (`GameplayStatics.GetPlayerCharacter` 0)))
  (set `self.PlayerRef` _asbp_character))

(event `self.Box.OnComponentBeginOverlap`
  (params (OverlappedComponent :type "PrimitiveComponent Object Reference") (OtherActor :type "Actor Object Reference") (OtherComp :type "PrimitiveComponent Object Reference") (OtherBodyIndex :type Integer) (bFromSweep :type Boolean) (SweepResult :type "HitResult Structure (by ref)"))
  (bind _asbp_character (cast `/Game/Blueprints/BP_Character` OtherActor))
  (`/Engine/EditorBlueprintResources/StandardMacros.IncrementInt` (`/Game/Blueprints/BP_Character.Pickups` _asbp_character)
    (:`  `
      (`self.K2_DestroyActor`))))

(fn `UserConstructionScript`)