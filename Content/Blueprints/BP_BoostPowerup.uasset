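; BP_BoostPowerup is a spinning pickup that grants the player character a boost power-up.
; BeginPlay caches the player's BP_Character, and Tick rotates the Rot component around its yaw axis by a fixed per-frame step.
; When a BP_Character overlaps the Box, it sets that character's HasBoostPU flag, turns the cached player's TimerHUD BoostText opaque white, then destroys itself.
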(event `self.ReceiveTick`
  (params (DeltaSeconds :type "Float (single-precision)"))
  (`SceneComponent.K2_AddRelativeRotation` (`self.Rot`) (struct :`Yaw` 2.0) false false))

(event `self.ReceiveBeginPlay`
  (bind _asbp_character (cast `/Game/Blueprints/BP_Character` (`GameplayStatics.GetPlayerCharacter` 0)))
  (set `self.PlayerRef` _asbp_character))

(event `self.Box.OnComponentBeginOverlap`
  (params (OverlappedComponent :type "PrimitiveComponent Object Reference") (OtherActor :type "Actor Object Reference") (OtherComp :type "PrimitiveComponent Object Reference") (OtherBodyIndex :type Integer) (bFromSweep :type Boolean) (SweepResult :type "HitResult Structure (by ref)"))
  (bind _asbp_character (cast `/Game/Blueprints/BP_Character` OtherActor))
  (set `/Game/Blueprints/BP_Character.HasBoostPU` true _asbp_character)
  (`TextBlock.SetColorAndOpacity` (`/Game/Blueprints/W_Timer.BoostText` (`/Game/Blueprints/BP_Character.TimerHUD` (`self.PlayerRef`))) (make `SlateColor` (make `LinearColor` 1.0 1.0 1.0 1.0)))
  (`self.K2_DestroyActor`))

(fn `UserConstructionScript`)