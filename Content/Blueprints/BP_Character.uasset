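; Player character for a timed level that switches between first-person-style walking and momentum-based flight.
; Flight inherits current speed and steers an arrow component that eases toward the camera, setting velocity with constant decay and added gravity.
; BP_Loop overlaps add speed, while low speed or collisions restore walking.
; It also drives FOV transitions, camera shakes, post-process, HUD, a looping timer counter and the finish-line completion screen.
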(event `InputAxis|MoveForward`
  (params (AxisValue :type "Float (single-precision)"))
  ;[1 1 1] Move & Look
  (if (not (`NavMovementComponent.IsFlying` (`self.CharacterMovement`)))
    (`self.AddMovementInput` (`self.GetActorForwardVector`) AxisValue)))

(event `InputAxis|MoveRight`
  (params (AxisValue :type "Float (single-precision)"))
  ;[1 1 1] Move & Look
  (if (not (`NavMovementComponent.IsFlying` (`self.CharacterMovement`)))
    (`self.AddMovementInput` (`self.GetActorRightVector`) AxisValue)))

(event `InputAxis|LookHorizontal`
  (params (AxisValue :type "Float (single-precision)"))
  ;[1 1 1] Move & Look
  (`self.AddControllerYawInput` AxisValue))

(event `InputAxis|LookVertical`
  (params (AxisValue :type "Float (single-precision)"))
  ;[1 1 1] Move & Look
  (`SceneComponent.K2_AddRelativeRotation` (`self.Camera`) (`KismetMathLibrary.MakeRotator` 0.0 AxisValue) false false))

(event `InputAction|Jump`
  (params (Key :type "Key Structure"))
  ;[1 1 1] Move & Look
  (:`Pressed`
    (`self.Jump`))
  (:`Released`
    (`self.StopJumping`)))

(event `InputAction|FlightToggle`
  (params (Key :type "Key Structure"))
  (bind _returnvalue (`self.GetVelocity`))
  (bind _charactermovement (`self.CharacterMovement`))
  (bind _returnvalue_2 (`KismetMathLibrary.VSize` _returnvalue))
  ;[1 1 1] Press LMB
  (:`Pressed`
    (if (`NavMovementComponent.IsFlying` (`self.CharacterMovement`))
      ;[1 1 1] Transition to walking
      (`CharacterMovementComponent.SetMovementMode` _charactermovement "MOVE_Walking" 0 :!label _label)
      (set `PostProcessComponent.bEnabled` false (`self.PostProcess`))
      (bind (_direction _newtrack_0) (`Timeline|StopFlying` :!via `PlayFromStart`)
        (:`Update`
          (set `self.FOVCurrent` (`KismetMathLibrary.Lerp` (`self.FOVFlying`) (`self.FOVWalking`) _newtrack_0))))
      (else
        ;[1 1 1] Transition to flying
        (`CharacterMovementComponent.SetMovementMode` _charactermovement "MOVE_Flying" 0)
        (set `self.CurrentSpeed` _returnvalue_2)
        (`KismetSystemLibrary.PrintString` (`KismetStringLibrary.Conv_DoubleToString` _returnvalue_2))
        (`SceneComponent.K2_SetWorldRotation` (`self.Arrow1`) (`KismetMathLibrary.Conv_VectorToRotator` _returnvalue) false false)
        (set `PostProcessComponent.bEnabled` true (`self.PostProcess`))
        (bind (_direction_2 _newtrack_0_2) (`Timeline|BeginFly` :!via `PlayFromStart`)
          (:`Update`
            (set `self.FOVCurrent` (`KismetMathLibrary.Lerp` (`self.FOVWalking`) (`self.FOVFlying`) _newtrack_0_2))))))))

(event `self.ReceiveTick`
  (params (DeltaSeconds :type "Float (single-precision)"))
  ;[1 1 1] Lerp arrow towards camera
  (`SceneComponent.K2_SetWorldRotation` (`self.Arrow1`) (`KismetMathLibrary.RInterpTo` (`SceneComponent.K2_GetComponentRotation` (`self.Arrow1`)) (`SceneComponent.K2_GetComponentRotation` (`self.Camera`)) DeltaSeconds 3.0) false false)
  ;[1 1 1] FOV
  (`CameraComponent.SetFieldOfView` (`self.Camera`) (`self.FOVCurrent`))
  ;[1 1 1] Decelerate
  (set `self.CurrentSpeed` (`KismetMathLibrary.FClamp` (- (`self.CurrentSpeed`) (`self.Dec`)) 0.0 (`self.MaxSpeed`)))
  ;[1 1 1] Cam shakes
  (`self.FlyShake`)
  (`self.Headbob`)
  ;[1 1 1] Is player flying?
  (if (`NavMovementComponent.IsFlying` (`self.CharacterMovement`))
    ;[1 1 1] Fly in direction of arrow
    (set `MovementComponent.Velocity` (+ (* (`SceneComponent.GetForwardVector` (`self.Arrow1`)) (`self.CurrentSpeed`)) (`KismetMathLibrary.MakeVector` 0.0 0.0 (`self.FlyGravity`))) (`self.CharacterMovement`))
    ;[1 1 1] Stop flying if too slow
    (if (<= (`self.CurrentSpeed`) (`self.MinFlySpeed`))
      (goto _label))))

(event `FlyShake`
  ;[1 1 1] Fly Shake
  (if (and (> (`KismetMathLibrary.VSize` (`self.GetVelocity`)) 0.0) (`NavMovementComponent.IsFlying` (`self.CharacterMovement`)))
    (`PlayerController.ClientStartCameraShake` :`self` (`GameplayStatics.GetPlayerController` 0) :`Shake` "/Game/Blueprints/BP_FlyShake.BP_FlyShake_C")))

(event `Headbob`
  ;[1 1 1] Headbob
  (if (and (> (`KismetMathLibrary.VSize` (`self.GetVelocity`)) 0.0) (`self.CanJump`))
    (`PlayerController.ClientStartCameraShake` :`self` (`GameplayStatics.GetPlayerController` 0) :`Shake` "/Game/Blueprints/BP_Headbob.BP_Headbob_C")))

(event `self.CapsuleComponent.OnComponentHit`
  (params (HitComponent :type "PrimitiveComponent Object Reference") (OtherActor :type "Actor Object Reference") (OtherComp :type "PrimitiveComponent Object Reference") (NormalImpulse :type "Vector Structure") (Hit :type "HitResult Structure (by ref)"))
  ;[1 1 1] Hit something = stop flying
  (if (`NavMovementComponent.IsFlying` (`self.CharacterMovement`))
    (goto _label)))

(event `self.ReceiveActorBeginOverlap`
  (params (OtherActor :type "Actor Object Reference"))
  ;[1 1 1] Flying through loop
  (cast `/Game/Blueprints/BP_Loop` OtherActor)
  (set `self.CurrentSpeed` (`KismetMathLibrary.FClamp` (+ (`self.CurrentSpeed`) (`self.Acc`)) 0.0 (`self.MaxSpeed`))))

(event `self.ReceiveBeginPlay`
  ;[1 1 1] Begin Play
  (bind _returnvalue (`|CreateWidget` "/Game/Blueprints/W_Sight.W_Sight_C"))
  (`UserWidget.AddToViewport` _returnvalue 0)
  (bind _output_get (set `self.HUD` _returnvalue))
  (set `PostProcessComponent.bEnabled` false (`self.PostProcess`))
  (`Widget.SetVisibility` (`/Game/Blueprints/W_Sight.BLOOD` _output_get) "Hidden")
  (bind _returnvalue_2 (`|CreateWidget` "/Game/Blueprints/W_Timer.W_Timer_C"))
  (`UserWidget.AddToViewport` _returnvalue_2 0)
  (`Timeline|Timeline_0` :!label _label_2
    (:`Finished`
      (`/Engine/EditorBlueprintResources/StandardMacros.IncrementInt` (`self.TimeLeft`)
        (:`  `
          (goto _label_2 :!via `PlayFromStart`))))))

(event `self.CapsuleComponent.OnComponentBeginOverlap`
  (params (OverlappedComponent :type "PrimitiveComponent Object Reference") (OtherActor :type "Actor Object Reference") (OtherComp :type "PrimitiveComponent Object Reference") (OtherBodyIndex :type Integer) (bFromSweep :type Boolean) (SweepResult :type "HitResult Structure (by ref)"))
  (bind _returnvalue (`GameplayStatics.GetPlayerController` 0))
  ;[1 1 1] Level Complete!
  (cast `/Game/Blueprints/BP_FinishLine` OtherActor)
  (`GameplayStatics.SetGamePaused` true)
  (set `PlayerController.bShowMouseCursor` true _returnvalue)
  (`WidgetBlueprintLibrary.SetInputMode_UIOnlyEx` _returnvalue null)
  (bind _returnvalue_2 (`|CreateWidget` "/Game/Blueprints/w_LevelComplete.W_LevelComplete_C"))
  (`UserWidget.AddToViewport` _returnvalue_2 0))

(fn `UserConstructionScript`)