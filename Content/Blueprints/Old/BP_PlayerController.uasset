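; An old player controller Blueprint whose logic is all disconnected, leaving BeginPlay and the construction script empty.
; The orphaned setup caches the first BP_Pawn and BP_Character found in the level and adds a W_Sight widget to the viewport.
; An orphaned FlipFlop swaps possession between them, moving the target to the other's location and rotation and copying camera rotation.
; Switching to the pawn also sets its speed to maximum and resets its FOV.
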(event `self.ReceiveBeginPlay`)

(event `InputAction|FlightToggle`
  (params (Key :type "Key Structure")))

(fn `UserConstructionScript`)