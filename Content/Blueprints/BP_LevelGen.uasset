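; BP_LevelGen is a level generator that scatters static mesh components through a 3D volume in its Construction Script.
; Nested X, Y and Z loops roll each cell against ChanceToSpawn to decide whether to add a mesh.
; Each mesh's position multiplies its indices by randomly scaled, truncated MeshDistance, giving an irregular layout, with slight random rotation and per-axis scale.
; The event graph is unused, and the unseeded randomness changes the layout on each reconstruction.
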(fn `UserConstructionScript`
  (bind _returnvalue (`KismetMathLibrary.FTrunc` (* (`self.MeshDistance`) (`KismetMathLibrary.RandomFloatInRange` 0.0 1.0))))
  (for _index (range (+ (`self.Z`) 1))
    (for _index_2 (range (+ (`self.Y`) 1))
      (for _index_3 (range (+ (`self.X`) 1))
        (if (< (`KismetMathLibrary.RandomFloatInRange` 0.0 100.0) (`self.ChanceToSpawn`))
          (`AddComponent|NODE_AddStaticMeshComponent-2` :`RelativeTransform` (`KismetMathLibrary.MakeTransform` (`KismetMathLibrary.MakeVector` (`KismetMathLibrary.Conv_IntToDouble` (* _index_3 _returnvalue)) (`KismetMathLibrary.Conv_IntToDouble` (* _index_2 _returnvalue)) (`KismetMathLibrary.Conv_IntToDouble` (* _index _returnvalue))) (`KismetMathLibrary.MakeRotator` (`KismetMathLibrary.RandomFloatInRange` -10.0 10.0) (`KismetMathLibrary.RandomFloatInRange` -10.0 10.0) (`KismetMathLibrary.RandomFloatInRange` -10.0 10.0)) (`KismetMathLibrary.MakeVector` (`KismetMathLibrary.RandomFloatInRange` 0.5 1.5) (`KismetMathLibrary.RandomFloatInRange` 0.5 1.5) (`KismetMathLibrary.RandomFloatInRange` 0.5 1.5)))))))))