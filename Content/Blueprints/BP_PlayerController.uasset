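; Player controller that lets the player toggle between a walking character and a flying pawn.
; On BeginPlay it caches the first BP_Pawn and BP_Character found in the level and adds the W_Sight widget to the viewport.
; The FlightToggle input drives a FlipFlop that moves the target body to the current one's transform, possesses it and copies camera rotation.
; Entering flight also sets the pawn to max speed and resets its FOV.
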(event `self.ReceiveBeginPlay`
  ;[1 1 1] Get Pawn & Character references
  (bind _outactors (`GameplayStatics.GetAllActorsOfClass` "/Game/Blueprints/BP_Pawn.BP_Pawn_C"))
  (set `self.PawnRef` (`|GetArrayItem` _outactors))
  (bind _outactors_2 (`GameplayStatics.GetAllActorsOfClass` "/Game/Blueprints/BP_Character.BP_Character_C"))
  (set `self.CharRef` (`|GetArrayItem` _outactors_2))
  (bind _returnvalue (`|CreateWidget` "/Game/Blueprints/W_Sight.W_Sight_C"))
  (`UserWidget.AddToViewport` _returnvalue 0))

(event `InputAction|FlightToggle`
  (params (Key :type "Key Structure"))
  (bind _charref (`self.CharRef`))
  (bind _pawnref (`self.PawnRef`))
  (bind _spherecollider (`/Game/Blueprints/BP_Pawn.SphereCollider` (`self.PawnRef`)))
  (bind _capsulecomponent (`Character.CapsuleComponent` (`self.CharRef`)))
  (:`Pressed`
    (`/Engine/EditorBlueprintResources/StandardMacros.FlipFlop`
      (:`A`
        (`SceneComponent.K2_SetWorldLocationAndRotation` (`/Game/Blueprints/BP_Pawn.SphereCollider` (`self.PawnRef`)) (`SceneComponent.K2_GetComponentLocation` _capsulecomponent) (`SceneComponent.K2_GetComponentRotation` _capsulecomponent) false false)
        (`self.Possess` _pawnref)
        (set `/Game/Blueprints/BP_Pawn.CurrentSpeed` (`/Game/Blueprints/BP_Pawn.MaxSpeed` _pawnref) _pawnref)
        (set `/Game/Blueprints/BP_Pawn.FOVCurrent` 90.0 _pawnref)
        (`SceneComponent.K2_SetWorldRotation` (`/Game/Blueprints/BP_Pawn.Camera` _pawnref) (`SceneComponent.K2_GetComponentRotation` (`/Game/Blueprints/BP_Character.Camera` (`self.CharRef`))) false false))
      (:`B`
        (`SceneComponent.K2_SetWorldLocationAndRotation` (`Character.CapsuleComponent` (`self.CharRef`)) (`SceneComponent.K2_GetComponentLocation` _spherecollider) (`SceneComponent.K2_GetComponentRotation` _spherecollider) false false)
        (`self.Possess` _charref)
        (`SceneComponent.K2_SetWorldRotation` (`/Game/Blueprints/BP_Character.Camera` _charref) (`SceneComponent.K2_GetComponentRotation` (`/Game/Blueprints/BP_Pawn.Camera` (`self.PawnRef`))) false false)))))

(fn `UserConstructionScript`)