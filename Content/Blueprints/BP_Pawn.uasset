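; Player pawn for a flying game in which passing through BP_Loop actors restores speed.
; Every tick it bleeds off speed, pitches the camera and yaws the sphere collider from input, then sweeps along the camera's forward vector under constant downward drift, without delta-time scaling.
; Overlapping a loop adds clamped speed and plays a timeline that drives camera FOV.
; R opens Level1; a Flying-based movement branch is left disconnected.
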(event `self.ReceiveTick`
  (params (DeltaSeconds :type "Float (single-precision)"))
  ;[1 1 1] FOV
  (`CameraComponent.SetFieldOfView` (`self.Camera`) (`self.FOVCurrent`))
  (set `self.CurrentSpeed` (`KismetMathLibrary.FClamp` (- (`self.CurrentSpeed`) (`self.Decel`)) 0.0 (`self.MaxSpeed`)))
  (`SceneComponent.K2_AddLocalRotation` (`self.Camera`) (`KismetMathLibrary.MakeRotator` 0.0 (`self.GetInputAxisValue`)) false false)
  (`SceneComponent.K2_AddLocalRotation` (`self.SphereCollider`) (`KismetMathLibrary.MakeRotator` 0.0 0.0 (`self.GetInputAxisValue`)) false false)
  ;[1 1 1] Fly forward
  (`SceneComponent.K2_AddWorldOffset` (`self.SphereCollider`) (* (`SceneComponent.GetForwardVector` (`self.Camera`)) (`self.CurrentSpeed`)) true false)
  ;[1 1 1] Gravity
  (`SceneComponent.K2_AddWorldOffset` (`self.SphereCollider`) (0.0 0.0 -5.0) false false))

(event `self.ReceiveActorBeginOverlap`
  (params (OtherActor :type "Actor Object Reference"))
  (cast `/Game/Blueprints/BP_Loop` OtherActor)
  (set `self.CurrentSpeed` (`KismetMathLibrary.FClamp` (+ (`self.CurrentSpeed`) (`self.Acc`)) 0.0 (`self.MaxSpeed`)))
  (bind (_direction _dist) (`Timeline|BoostFOV` :`NewTime` 2.0 :!via `PlayFromStart`)
    (:`Update`
      (set `self.FOVCurrent` _dist))))

(event `self.ReceiveBeginPlay`
  (set `self.CurrentSpeed` (`self.MaxSpeed`)))

(event `Key|R`
  (params (Key :type "Key Structure"))
  (:`Pressed`
    (`GameplayStatics.OpenLevel` "Level1")))

(fn `UserConstructionScript`)